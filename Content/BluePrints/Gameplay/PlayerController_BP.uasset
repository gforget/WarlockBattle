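; Player controller that passes directional movement input on to the player's Warlock character.
; On BeginPlay it casts player character 0 to Warlock_BP and caches the reference.
; Separate Forward, Backward, Right and Left axis events each pass their value to the matching move function on the Warlock, which handles the movement itself.
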(event EventBeginPlay
  (Variables|Default|SetWarlock (.AsWarlock%20BP (Utilities|Casting|CastToWarlock_BP (Game|GetPlayerCharacter 0)))))

(event Input|AxisEvents|InputAxisBackward
  (params (AxisValue :type Float%20%28single-precision%29))
  (Default|MoveBackward (Variables|Default|GetWarlock) AxisValue))

(event Input|AxisEvents|InputAxisForward
  (params (AxisValue :type Float%20%28single-precision%29))
  (Default|MoveForward (Variables|Default|GetWarlock) AxisValue))

(event Input|AxisEvents|InputAxisRight
  (params (AxisValue :type Float%20%28single-precision%29))
  (Default|MoveRight (Variables|Default|GetWarlock) AxisValue))

(event Input|AxisEvents|InputAxisLeft
  (params (AxisValue :type Float%20%28single-precision%29))
  (Default|MoveLeft (Variables|Default|GetWarlock) AxisValue))

(fn ConstructionScript)