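; Warlock character Blueprint that handles planar movement and facing from four directional intensity events.
; The MoveForward, MoveBackward, MoveRight and MoveLeft events store intensities, which Tick sums into a world X/Y direction.
; Tick writes CharacterMovement velocity directly as that normalized direction, scaled by clamped input magnitude and Speed.
; While moving, it rotates only the mesh toward the velocity via a look-at rotation combined with RotationCorrector.
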(event Custom|MoveForward
  (params (intensity :type Float%20%28single-precision%29))
  (Variables|Default|SetForward intensity))

(event Custom|MoveBackward
  (params (intensity :type Float%20%28single-precision%29))
  (Variables|Default|SetBackward intensity))

(event Custom|MoveRight
  (params (intensity :type Float%20%28single-precision%29))
  (Variables|Default|SetRight intensity))

(event Custom|MoveLeft
  (params (intensity :type Float%20%28single-precision%29))
  (Variables|Default|SetLeft intensity))

(event EventTick
  (params (DeltaSeconds :type Float%20%28single-precision%29))
  (bind _returnvalue (Transformation|GetActorLocation))
  (bind _forward (Variables|Default|GetForward))
  (bind _backward (Variables|Default|GetBackward))
  (bind _right (Variables|Default|GetRight))
  (bind _left (Variables|Default|GetLeft))
  (bind _returnvalue_2 (+ _right _left))
  (bind _returnvalue_3 (+ _forward _backward))
  (Variables|Default|SetForwardIntensity (Math|Float|Absolute(Float) _returnvalue_3))
  (Variables|Default|SetRightIntensity (Math|Float|Absolute(Float) _returnvalue_2))
  (bind _output_get (Variables|Default|SetCurrentVelocity (Math|Vector|MakeVector _returnvalue_3 _returnvalue_2 0.0)))
  (bind _output_get_2 (Variables|/Script/Engine.MovementComponent|SetVelocity (Variables|Character|GetCharacterMovement) (* (Math|Vector|Normalize _output_get) (* (Math|Float|Clamp(Float) (+ (Variables|Default|GetRightIntensity) (Variables|Default|GetForwardIntensity))) (Variables|Default|Getspeed)))))
  (if (!= (Math|Vector|VectorLength _output_get_2) 0.0)
    (Transformation|SetWorldRotation (Variables|Character|GetMesh) (Math|Rotator|CombineRotators (Math|Rotator|FindLookatRotation _returnvalue (+ _output_get_2 _returnvalue)) (Variables|Default|GetrotationCorrector)) false false)))

(fn ConstructionScript)